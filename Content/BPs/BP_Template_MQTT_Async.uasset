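; Template actor demonstrating the asynchronous Paho MQTT client plugin against a HiveMQ broker.
; On BeginPlay it spawns an MQTT_Manager_Paho_Async, initializes it with server and credentials from the GI_Plugins game instance, then binds delegates for arrived, delivered, lost, connect and send events.
; The connect callback publishes a test message and subscribes to a web topic.
; Results and callbacks are printed on screen, mostly color-coded green or red by outcome.
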(event `Delegate_OnSend_Event`
  (params (Out_Result :type "JsonObjectWrapper Structure"))
  (bind _outvalue (`|GetJsonField` Out_Result "Payload"))
  (`KismetSystemLibrary.PrintString` _outvalue))

(event `self.ReceiveBeginPlay`
  (bind _asgi_plugins (cast `/Game/Player/GI_Plugins` (`GameplayStatics.GetGameInstance`)))
  (set `self.REF_GI_Plugins` _asgi_plugins)
  (bind _returnvalue (`|SpawnActorFromClass` "/Script/FF_MQTT_Async.MQTT_Manager_Paho_Async" (`KismetMathLibrary.MakeTransform` (0.0 0.0 0.0)) "Undefined" "MultiplyWithRoot" null null))
  (bind _output_get (set `self.REF_Paho_Async` _returnvalue))
  (bind (_out_code _returnvalue_2) (`MQTT_Manager_Paho_Async.MQTT_Async_Init` _output_get (make `PahoClientParams` "UE5_Paho_C_Async" (`BlueprintMapLibrary.Map_Find` (`/Game/Player/GI_Plugins.Servers` (`self.REF_GI_Plugins`)) "hivemq") (`BlueprintMapLibrary.Map_Find` (`/Game/Player/GI_Plugins.Users` (`self.REF_GI_Plugins`)) "hivemq") (`BlueprintMapLibrary.Map_Find` (`/Game/Player/GI_Plugins.Passwords` (`self.REF_GI_Plugins`)) "hivemq"))))
  (bind _outvalue (`|GetJsonField` _out_code "ErrorCode"))
  (bind _outvalue_2 (`|GetJsonField` _out_code "Description"))
  (`KismetSystemLibrary.PrintString` (`KismetStringLibrary.Concat_StrStr` _outvalue_2 " = " _outvalue) true true (select `bool` _returnvalue_2 :`false` (struct :`R` 1.0 :`A` 1.0) :`true` (struct :`G` 1.0 :`A` 1.0) :!type "LinearColor Structure") 30.0)
  (add `MQTT_Manager_Paho_Async.Delegate_Arrived` (`self.REF_Paho_Async`) (delegate `Delegate_Arrived_Event`))
  (add `MQTT_Manager_Paho_Async.Delegate_Delivered` (`self.REF_Paho_Async`) (delegate `Delegate_Delivered_Event`))
  (add `MQTT_Manager_Paho_Async.Delegate_Lost` (`self.REF_Paho_Async`) (delegate `Delegate_Lost_Event`))
  (add `MQTT_Manager_Paho_Async.Delegate_OnConnect` (`self.REF_Paho_Async`) (delegate `Delegate_OnConnect_Event`))
  (add `MQTT_Manager_Paho_Async.Delegate_OnSend` (`self.REF_Paho_Async`) (delegate `Delegate_OnSend_Event`)))

(event `Delegate_Arrived_Event`
  (params (Out_Result :type "PahoArrived Structure"))
  (`KismetSystemLibrary.PrintString` (`KismetStringLibrary.Concat_StrStr` Out_Result_Message " = " Out_Result_TopicName) true true (struct :`G` 1.0 :`A` 1.0) 30.0))

(event `Delegate_Delivered_Event`
  (params (Out_Result :type String))
  (`KismetSystemLibrary.PrintString` Out_Result true true (struct :`G` 1.0 :`A` 1.0) 30.0))

(event `Delegate_Lost_Event`
  (params (Out_Cause :type String))
  (`KismetSystemLibrary.PrintString` "Hello" true true (struct :`R` 1.0 :`A` 1.0) 30.0))

(event `Delegate_OnConnect_Event`
  (params (Out_Result :type "JsonObjectWrapper Structure"))
  (bind (_out_code _returnvalue) (`MQTT_Manager_Paho_Async.MQTT_Async_Publish` (`self.REF_Paho_Async`) "ue5_async" "This message sent from UE5 with Async client plugin." "QoS_0" 0))
  (bind _outvalue (`|GetJsonField` _out_code "ErrorCode"))
  (bind _outvalue_2 (`|GetJsonField` _out_code "Description"))
  (`KismetSystemLibrary.PrintString` (`KismetStringLibrary.Concat_StrStr` _outvalue_2 " = " _outvalue) true true (select `bool` _returnvalue :`false` (struct :`R` 1.0 :`A` 1.0) :`true` (struct :`G` 1.0 :`A` 1.0) :!type "LinearColor Structure") 30.0)
  (bind (_out_code_2 _returnvalue_2) (`MQTT_Manager_Paho_Async.MQTT_Async_Subscribe` (`self.REF_Paho_Async`) "web" "QoS_0"))
  (bind _outvalue_3 (`|GetJsonField` _out_code_2 "ErrorCode"))
  (bind _outvalue_4 (`|GetJsonField` _out_code_2 "Description"))
  (`KismetSystemLibrary.PrintString` (`KismetStringLibrary.Concat_StrStr` _outvalue_4 " = " _outvalue_3) true true (select `bool` _returnvalue_2 :`false` (struct :`R` 1.0 :`A` 1.0) :`true` (struct :`G` 1.0 :`A` 1.0) :!type "LinearColor Structure") 30.0))

(fn `UserConstructionScript`)